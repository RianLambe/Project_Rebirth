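; Reusable interactable door that the player can open once through a scripted first-person animation.
; On interact, it disables further interaction, freezes the player, snaps them to an offset relative to the door's rotated transform and hides their held item.
; It plays the arms montage alongside the door's skeletal animation, then restores movement and item visibility after a fixed delay rather than on montage completion.
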(event OnInteract(Interaction)
  (bind _returnvalue (Transformation|GetActorTransform))
  (if (not (Variables|Default|GetDoorOpen))
    (Variables|/Script/ProjectRebirth.Interaction|SetCanInteract (Variables|Default|GetInteraction) false)
    (Variables|Default|SetDoorOpen true)
    (bind _outactors (Actor|GetAllActorsOfClass "/Game/Characters/FirstPerson/Blueprints/Player.Player_C"))
    (bind _output_get (Variables|Default|SetPlayerRef (Utilities|Array|Get(acopy) _outactors)))
    (Class|ProjectRebirthCharacter|FreezePlayer _output_get true)
    (Class|ProjectRebirthCharacter|RelocatePlayer _output_get (Math|Transform|MakeTransform (.location _returnvalue) (Math|Rotator|MakeRotator (.roll (.rotation _returnvalue)) (.pitch (.rotation _returnvalue)) (+ (.yaw (.rotation _returnvalue)) 2.7e+02)) (.scale _returnvalue)) (Math|Transform|MakeTransform "-50.000000,0.000000,50.000000" "0, 0, 0" "1.000000,1.000000,1.000000"))
    (Rendering|SetVisibility (Variables|/Script/ProjectRebirth.ProjectRebirthCharacter|GetItemMesh _output_get) false false)
    (Animation|Montage|PlayMontage (Variables|/Script/ProjectRebirth.ProjectRebirthCharacter|GetFPArmsMesh _output_get) "/Game/PlayerModels/Animations/Arms_Door_OpenOutside_Montage.Arms_Door_OpenOutside_Montage"
      (:then
        (Components|Animation|PlayAnimation (Variables|SkeletalMeshActor|GetSkeletalMeshComponent) "/Game/Enviroment/Door/Door_Open.Door_Open" false)
        (Utilities|FlowControl|Delay 2.33)
        (Class|ProjectRebirthCharacter|FreezePlayer (Variables|Default|GetPlayerRef) false)
        (Rendering|SetVisibility (Variables|/Script/ProjectRebirth.ProjectRebirthCharacter|GetItemMesh _output_get) true false)))))

(fn ConstructionScript)